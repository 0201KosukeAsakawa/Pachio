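; Double door for the Ancient Temple Ruins set that swings open when an actor enters its trigger volume and closes when it leaves.
; The DoorRotationSpeed timeline plays on overlap and reverses on exit, with two tracks scaled by RotationAngle2 setting each leaf's relative yaw.
; Both overlap events filter through a placeholder cast to Controller, marked for replacement with the project's character controller.
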(event OnComponentBeginOverlap(Trigger_Volume)
  (params (OverlappedComponent :type Primitive%20Component%20Object%20Reference) (OtherActor :type Actor%20Object%20Reference) (OtherComp :type Primitive%20Component%20Object%20Reference) (OtherBodyIndex :type Integer) (bFromSweep :type Boolean) (SweepResult :type Hit%20Result%20Structure%20%28by%20ref%29))
  (bind _rotation_angle_2 (Variables|Default|GetRotation%20Angle%202))
  ;[1 1 1] Replace with your Character controller
  (Utilities|Casting|CastToController OtherActor)
  (bind (_direction _rotation _rottion_02) (Timeline|Timeline Play)
    (:Update
      (Transformation|SetRelativeRotation (Variables|Default|GetSM_Door_01_B) (Math|Rotator|MakeRotator 0.0 0.0 (* _rotation _rotation_angle_2)) false false)
      (Transformation|SetRelativeRotation (Variables|Default|GetSM_Door_01_B1) (Math|Rotator|MakeRotator 0.0 0.0 (* _rottion_02 _rotation_angle_2)) false false))))

(event OnComponentEndOverlap(Trigger_Volume)
  (params (OverlappedComponent :type Primitive%20Component%20Object%20Reference) (OtherActor :type Actor%20Object%20Reference) (OtherComp :type Primitive%20Component%20Object%20Reference) (OtherBodyIndex :type Integer))
  (bind _rotation_angle_2 (Variables|Default|GetRotation%20Angle%202))
  ;[1 1 1] Replace with your Character controller
  (Utilities|Casting|CastToController OtherActor)
  (bind (_direction _rotation _rottion_02) (Timeline|Timeline Reverse)
    (:Update
      (Transformation|SetRelativeRotation (Variables|Default|GetSM_Door_01_B) (Math|Rotator|MakeRotator 0.0 0.0 (* _rotation _rotation_angle_2)) false false)
      (Transformation|SetRelativeRotation (Variables|Default|GetSM_Door_01_B1) (Math|Rotator|MakeRotator 0.0 0.0 (* _rottion_02 _rotation_angle_2)) false false))))

(event EventBeginPlay)

(event Collision|EventActorBeginOverlap
  (params (OtherActor :type Actor%20Object%20Reference)))

(event EventTick
  (params (DeltaSeconds :type Float%20%28single-precision%29)))

(fn ConstructionScript)